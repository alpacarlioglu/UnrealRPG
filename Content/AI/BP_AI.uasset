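; Enemy character Blueprint that takes damage, dies into a ragdoll and can be stealth-assassinated by the player.
; AnyDamage plays a random hit montage, launches it along the player's facing, and decreases health through BPPlayerStatsNew, ragdolling on death.
; An overlap radius toggles the assassinate prompt; StealthBackAssassin plays the victim montage, triggers delayed ragdoll and returns alignment transforms.
; Tick turns the health bar toward the camera; Attack is a stub.
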(event `self.ReceiveBeginPlay`
  (bind _aswb_dummy_health (cast `/Game/UI/WB_DummyHealth` (`WidgetComponent.GetWidget` (`self.Health Bar`))))
  (set `self.Health Bar WidgetBP` _aswb_dummy_health))

(event `self.ReceiveTick`
  (params (DeltaSeconds :type "Float (single-precision)"))
  (bind _health_bar (`self.Health Bar`))
  (`SceneComponent.K2_SetWorldRotation` _health_bar (`KismetMathLibrary.FindLookAtRotation` (`SceneComponent.K2_GetComponentLocation` _health_bar) (`SceneComponent.K2_GetComponentLocation` (`PlayerCameraManager.TransformComponent` (`GameplayStatics.GetPlayerCameraManager` 0)))) false false))

(event `Ragdoll`
  ;[0.05127 0.05127 0.05127] Ragdoll
  (`|ExecutionSequence`
    (:`then_0`
      (`KismetSystemLibrary.Delay` 2.0)
      (`PrimitiveComponent.SetSimulatePhysics` (`self.Mesh`) true))
    (:`then_1`
      (`KismetSystemLibrary.Delay` 1.7)
      (`GameplayStatics.PlaySoundAtLocation` "/Game/Audio/Grunts-Hit/SC_Death.SC_Death" (`self.K2_GetActorLocation`) (struct) 1.0 1.0 0.0 "/Game/Audio/SA_Character.SA_Character" null null null))))

(event `self.Assassination Radius.OnComponentBeginOverlap`
  (params (OverlappedComponent :type "PrimitiveComponent Object Reference") (OtherActor :type "Actor Object Reference") (OtherComp :type "PrimitiveComponent Object Reference") (OtherBodyIndex :type Integer) (bFromSweep :type Boolean) (SweepResult :type "HitResult Structure (by ref)"))
  (cast `/Game/Blueprints/BP_ThirdPersonCharacter` OtherActor)
  (`SceneComponent.SetVisibility` (`self.Assassinate Widget`) true false))

(event `self.Assassination Radius.OnComponentEndOverlap`
  (params (OverlappedComponent :type "PrimitiveComponent Object Reference") (OtherActor :type "Actor Object Reference") (OtherComp :type "PrimitiveComponent Object Reference") (OtherBodyIndex :type Integer))
  (cast `/Game/Blueprints/BP_ThirdPersonCharacter` OtherActor)
  (`SceneComponent.SetVisibility` (`self.Assassinate Widget`) false false))

(event `self.ReceiveAnyDamage`
  (params (Damage :type "Float (single-precision)") (DamageType :type "DamageType Object Reference") (InstigatedBy :type "Controller Object Reference") (DamageCauser :type "Actor Object Reference"))
  (`self.PlayAnimMontage` (`KismetArrayLibrary.Array_Random` (`self.Hit Anims`)))
  (bind _asbp_third_person_character (cast `/Game/Blueprints/BP_ThirdPersonCharacter` (`GameplayStatics.GetPlayerCharacter` 0)))
  (`self.LaunchCharacter` (* (`KismetMathLibrary.GetForwardVector` (`self.K2_GetActorRotation` _asbp_third_person_character)) 700.0))
  (`GameplayStatics.PlaySoundAtLocation` "/Game/Audio/Grunts-Hit/416838__tonsil5__grunt2-death-pain.416838__tonsil5__grunt2-death-pain" (`self.K2_GetActorLocation`) (struct) 1.0 (`KismetMathLibrary.RandomFloatInRange` -0.5 0.5) 0.0 "/Game/Audio/SA_Character.SA_Character" null null null)
  (bind _is_player_death (`/Game/Blueprints/BP_PlayerStatsNew.Decrease Health` (`self.BP_PlayerStatsNew`) Damage))
  (if _is_player_death
    (`PrimitiveComponent.SetSimulatePhysics` (`self.Mesh`) true)
    (`SceneComponent.SetVisibility` (`self.Health Bar`) false false)
    (`GameplayStatics.PlaySoundAtLocation` "/Game/Audio/Grunts-Hit/SC_Death.SC_Death" (`self.K2_GetActorLocation`) (struct) 1.0 1.0 0.0 null null null null)
    (`SceneComponent.SetVisibility` (`self.Health Bar`) false false)))

(fn `Attack`
  (returns (`Animation Duration` :type "Float (double-precision)"))
  (return 0.0))

(fn `Stealth Back Assassin`
  (returns (`REF Location` :type "Vector Structure") (`Assassin Rotation` :type "Rotator Structure"))
  (`self.PlayAnimMontage` "/Game/Characters/RPG_Character/Animations/Assassinations/Paired_Knife_Stealth_KidneyAndNeck_Vic_Montage.Paired_Knife_Stealth_KidneyAndNeck_Vic_Montage")
  (`self.Ragdoll`)
  (`SceneComponent.SetVisibility` (`self.Assassinate Widget`) false false)
  (return (`SceneComponent.K2_GetComponentLocation` (`self.Assasin REF`)) (`self.K2_GetActorRotation`)))

(fn `UserConstructionScript`)