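; Stats component for the player character or a training dummy, tracking health, plus stamina, XP and level for the player.
; BeginPlay waits a tick, casts the owner to set IsPlayer, then fills the player HUD or dummy health bar.
; Stat functions update widgets directly; decreases return true on depletion, and only health damage supports the dummy's widget.
; Level-up is unwired: IncreaseXP never calls IncreaseLevel, whose logic is disconnected.
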(event `self.ReceiveBeginPlay`
  (`KismetSystemLibrary.DelayUntilNextTick`)
  (bind _asbp_third_person_character (cast `/Game/Blueprints/BP_ThirdPersonCharacter` (`self.GetOwner`))
    (:`then`
      (set `self.Player Character BP` _asbp_third_person_character)
      (set `self.Is Player?` true)
      (`ProgressBar.SetPercent` (`/Game/UI/WB_HUD.StaminaBar` (`/Game/Blueprints/BP_ThirdPersonCharacter.HUD Widget` (`self.Player Character BP`))) (/ (`self.Current Stamina`) (`self.Max Stamina`))))
    (:`CastFailed`
      (bind _asbp_dummy (cast `/Game/Blueprints/BP_Dummy` (`self.GetOwner`)))
      (set `self.Dummy BP` _asbp_dummy)
      (set `self.Is Player?` false)))
  (`ProgressBar.SetPercent` (select `bool` (`self.Is Player?`) :`false` (`/Game/UI/WB_DummyHealth.HealthBar` (`/Game/Blueprints/BP_Dummy.Health Bar WidgetBP` (`self.Dummy BP`))) :`true` (`/Game/UI/WB_HUD.HealthBar` (`/Game/Blueprints/BP_ThirdPersonCharacter.HUD Widget` (`self.Player Character BP`)))) (/ (`self.Current Health`) (`self.Max Health`)))
  (`TextBlock.SetText` (select `bool` (`self.Is Player?`) :`false` (`/Game/UI/WB_DummyHealth.DummyHealthText` (`/Game/Blueprints/BP_Dummy.Health Bar WidgetBP` (`self.Dummy BP`))) :`true` (`/Game/UI/WB_HUD.HealthText` (`/Game/Blueprints/BP_ThirdPersonCharacter.HUD Widget` (`self.Player Character BP`)))) (`KismetTextLibrary.Conv_DoubleToText` (`self.Current Health`) "HalfToEven"))
  (if (`self.Is Player?`)
    (`ProgressBar.SetPercent` (`/Game/UI/WB_HUD.XPBar` (`/Game/Blueprints/BP_ThirdPersonCharacter.HUD Widget` (`self.Player Character BP`))) (/ (`self.Current XP`) (`self.Max XP`)))
    (`TextBlock.SetText` (`/Game/UI/WB_HUD.XPText` (`/Game/Blueprints/BP_ThirdPersonCharacter.HUD Widget` (`self.Player Character BP`))) (`|FormatText` "{Current XP} / {Max XP}" (`self.Current XP`) (`self.Max XP`)))
    (`TextBlock.SetText` (`/Game/UI/WB_HUD.LevelText` (`/Game/Blueprints/BP_ThirdPersonCharacter.HUD Widget` (`self.Player Character BP`))) (`KismetTextLibrary.Conv_IntToText` (`self.Level`)))))

(fn `Decrease Health`
  (params (Damage :type "Float (double-precision)"))
  (returns (`Is Player Death` :type Boolean))
  (if (not (<= (`self.Current Health`) 0.0))
    (bind _output_get (set `self.Current Health` (- (`self.Current Health`) Damage)))
    (`ProgressBar.SetPercent` (select `bool` (`self.Is Player?`) :`false` (`/Game/UI/WB_DummyHealth.HealthBar` (`/Game/Blueprints/BP_Dummy.Health Bar WidgetBP` (`self.Dummy BP`))) :`true` (`/Game/UI/WB_HUD.HealthBar` (`/Game/Blueprints/BP_ThirdPersonCharacter.HUD Widget` (`self.Player Character BP`)))) (/ _output_get (`self.Max Health`)))
    (`TextBlock.SetText` (select `bool` (`self.Is Player?`) :`false` (`/Game/UI/WB_DummyHealth.DummyHealthText` (`/Game/Blueprints/BP_Dummy.Health Bar WidgetBP` (`self.Dummy BP`))) :`true` (`/Game/UI/WB_HUD.HealthText` (`/Game/Blueprints/BP_ThirdPersonCharacter.HUD Widget` (`self.Player Character BP`)))) (`KismetTextLibrary.Conv_DoubleToText` (`self.Current Health`) "HalfToEven"))
    (if (<= (`self.Current Health`) 0.0)
      _
      (else
        (return false))))
  (return true))

(fn `Decrease Stamina`
  (params (`Decrease Stamina` :type "Float (double-precision)"))
  (returns (`No Stamina Left` :type Boolean))
  (if (not (<= (`self.Current Stamina`) 0.0))
    (set `self.Current Stamina` (- (`self.Current Stamina`) `Decrease Stamina`))
    (`ProgressBar.SetPercent` (`/Game/UI/WB_HUD.StaminaBar` (`/Game/Blueprints/BP_ThirdPersonCharacter.HUD Widget` (`self.Player Character BP`))) (/ (`self.Current Stamina`) (`self.Max Stamina`)))
    (if (<= (`self.Current Stamina`) 0.0)
      _
      (else
        (return false))))
  (return true))

(fn `Increase Health`
  (params (`Health Increase` :type "Float (double-precision)"))
  (bind _hud_widget (`/Game/Blueprints/BP_ThirdPersonCharacter.HUD Widget` (`self.Player Character BP`)))
  (set `self.Current Health` (+ (`self.Current Health`) `Health Increase`))
  (if (> (`self.Current Health`) (`self.Max Health`))
    (set `self.Current Health` (`self.Max Health`)))
  (`ProgressBar.SetPercent` (`/Game/UI/WB_HUD.HealthBar` _hud_widget) (/ (`self.Current Health`) (`self.Max Health`)))
  (`TextBlock.SetText` (`/Game/UI/WB_HUD.HealthText` _hud_widget) (`KismetTextLibrary.Conv_DoubleToText` (`self.Current Health`) "HalfToEven")))

(fn `Increase Level`
  (params (B :type Integer)))

(fn `Increase Max Health`
  (params (`Max Health Increase` :type "Float (double-precision)"))
  (bind _hud_widget (`/Game/Blueprints/BP_ThirdPersonCharacter.HUD Widget` (`self.Player Character BP`)))
  (set `self.Max Health` (+ (`self.Max Health`) `Max Health Increase`))
  (`ProgressBar.SetPercent` (`/Game/UI/WB_HUD.HealthBar` _hud_widget) (/ (`self.Current Health`) (`self.Max Health`)))
  (`TextBlock.SetText` (`/Game/UI/WB_HUD.HealthText` _hud_widget) (`KismetTextLibrary.Conv_DoubleToText` (`self.Current Health`) "HalfToEven")))

(fn `Increase Max Stamina`
  (params (`Adding Stamina` :type "Float (double-precision)"))
  (set `self.Max Stamina` (+ (`self.Max Stamina`) `Adding Stamina`))
  (`ProgressBar.SetPercent` (`/Game/UI/WB_HUD.StaminaBar` (`/Game/Blueprints/BP_ThirdPersonCharacter.HUD Widget` (`self.Player Character BP`))) (/ (`self.Current Stamina`) (`self.Max Stamina`))))

(fn `Increase Stamina`
  (params (`Stamina Increase` :type "Float (double-precision)"))
  (set `self.Current Stamina` (+ (`self.Current Stamina`) `Stamina Increase`))
  (if (> (`self.Current Stamina`) (`self.Max Stamina`))
    (set `self.Current Stamina` (`self.Max Stamina`)))
  (`ProgressBar.SetPercent` (`/Game/UI/WB_HUD.StaminaBar` (`/Game/Blueprints/BP_ThirdPersonCharacter.HUD Widget` (`self.Player Character BP`))) (/ (`self.Current Stamina`) (`self.Max Stamina`))))

(fn `Increase XP`
  (params (`Recieving XP` :type "Float (double-precision)"))
  (set `self.Current XP` (+ (`self.Current XP`) `Recieving XP`))
  (if (not (>= (`self.Current XP`) (`self.Max XP`)))
    (`ProgressBar.SetPercent` (`/Game/UI/WB_HUD.XPBar` (`/Game/Blueprints/BP_ThirdPersonCharacter.HUD Widget` (`self.Player Character BP`))) (/ (`self.Current XP`) (`self.Max XP`)))
    (`TextBlock.SetText` (`/Game/UI/WB_HUD.XPText` (`/Game/Blueprints/BP_ThirdPersonCharacter.HUD Widget` (`self.Player Character BP`))) (`|FormatText` "{Current XP} / {Max XP}" (`self.Current XP`) (`self.Max XP`)))))